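; Bocce ball actor that colors itself to match a player's chosen color.
; On BeginPlay it looks up a PlayerCharacter_01 with GetActorOfClass and reads its PlayerColor enum.
; A branch chain then sets the static mesh's material to the red, blue, green or yellow variant.
; The color comes from whichever character that lookup returns, not from an owner or instigator reference.
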(event `self.ReceiveBeginPlay`
  (bind _returnvalue (`GameplayStatics.GetActorOfClass` "/Game/Character/Player/PlayerCharacter_01.PlayerCharacter_01_C"))
  (bind _playercolor (`/Game/Character/Player/PlayerCharacter_01.PlayerColor` _returnvalue))
  (if (`|EnumEquality` _playercolor "NewEnumerator2")
    (`PrimitiveComponent.SetMaterial` (`self.StaticMesh`) 0 "/Game/Balls/BocceBall_01/MI_BocceBall_01_Red.MI_BocceBall_01_Red")
    (elif (`|EnumEquality` _playercolor "NewEnumerator0")
      (`PrimitiveComponent.SetMaterial` (`self.StaticMesh`) 0 "/Game/Balls/BocceBall_01/MI_BocceBall_01_Blue.MI_BocceBall_01_Blue")
      (elif (`|EnumEquality` _playercolor "NewEnumerator1")
        (`PrimitiveComponent.SetMaterial` (`self.StaticMesh`) 0 "/Game/Balls/BocceBall_01/MI_BocceBall_01_Green.MI_BocceBall_01_Green")
        (elif (`|EnumEquality` _playercolor "NewEnumerator3")
          (`PrimitiveComponent.SetMaterial` (`self.StaticMesh`) 0 "/Game/Balls/BocceBall_01/MI_BocceBall_01_Yellow.MI_BocceBall_01_Yellow"))))))

(fn `UserConstructionScript`
  (`parent.UserConstructionScript`))