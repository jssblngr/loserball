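; Blue bocce ball Blueprint that reports its in-play status to BP_GameMode through IdiotBallSetup.
; On BeginPlay or UpdateInPlay it flags the stick, point ball and bocce ball all as true.
; When destroyed, it clears only the bocce flag, passing the current stick and point ball in-play values from BP_GameState.
; The construction script only calls the parent's.
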(event `UpdateInPlay`
  (bind _asbp_game_mode (cast `/Game/Blueprints/Gameplay/BP_GameMode` (`GameplayStatics.GetGameMode`)))
  (`/Game/Blueprints/Gameplay/BP_GameMode.IdiotBall_Setup` _asbp_game_mode true true true))

(event `self.ReceiveBeginPlay`
  (`self.UpdateInPlay`))

(event `self.ReceiveDestroyed`
  (bind _asbp_game_state (cast `/Game/Blueprints/Gameplay/BP_GameState` (`GameplayStatics.GetGameState`)))
  (bind _asbp_game_mode (cast `/Game/Blueprints/Gameplay/BP_GameMode` (`GameplayStatics.GetGameMode`)))
  (`/Game/Blueprints/Gameplay/BP_GameMode.IdiotBall_Setup` _asbp_game_mode (`/Game/Blueprints/Gameplay/BP_GameState.InPlay?_Stick` _asbp_game_state) (`/Game/Blueprints/Gameplay/BP_GameState.InPlay?_PointBall` _asbp_game_state) false))

(fn `UserConstructionScript`
  (`parent.UserConstructionScript`))