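; BP_PointBall_01 is a point ball actor among the golf ball assets that reports its in-play status to BP_GameMode.
; On BeginPlay it calls IdiotBallSetup with Stick and PointBall set and Bocce cleared.
; When destroyed, it clears PointBall through the same call, taking Stick and Bocce from BP_GameState.
; A DistanceToGolfBall event prints the 2D distance from its mesh to an actor of a given class.
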(event `UpdateInPlay`
  (bind _asbp_game_mode (cast `/Game/Blueprints/Gameplay/BP_GameMode` (`GameplayStatics.GetGameMode`)))
  (`/Game/Blueprints/Gameplay/BP_GameMode.IdiotBall_Setup` _asbp_game_mode true true false))

(event `self.ReceiveBeginPlay`
  (`self.UpdateInPlay`))

(event `DistanceTo GolfBall`
  (params (ActorClass :type "Actor Class Reference"))
  (bind _returnvalue (`GameplayStatics.GetActorOfClass` ActorClass))
  (`KismetSystemLibrary.PrintString` (`KismetStringLibrary.Conv_DoubleToString` (`KismetMathLibrary.Vector_Distance2D` (`SceneComponent.K2_GetComponentLocation` (`self.GetComponentByClass` _returnvalue "/Script/Engine.StaticMeshComponent")) (`SceneComponent.K2_GetComponentLocation` (`self.StaticMesh`)))) true true (struct :`G` 0.66 :`B` 1.0 :`A` 1.0) 30.0))

(event `self.ReceiveDestroyed`
  (bind _asbp_game_state (cast `/Game/Blueprints/Gameplay/BP_GameState` (`GameplayStatics.GetGameState`)))
  (bind _asbp_game_mode (cast `/Game/Blueprints/Gameplay/BP_GameMode` (`GameplayStatics.GetGameMode`)))
  (`/Game/Blueprints/Gameplay/BP_GameMode.IdiotBall_Setup` _asbp_game_mode (`/Game/Blueprints/Gameplay/BP_GameState.InPlay?_Stick` _asbp_game_state) false (`/Game/Blueprints/Gameplay/BP_GameState.InPlay?_BocceBall` _asbp_game_state)))

(fn `UserConstructionScript`
  (`parent.UserConstructionScript`))