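; Golf ball actor Blueprint with an event that reports how far the ball is from an actor of a given class.
; DistanceToGolfBall finds one actor of that class and measures the horizontal (2D) distance between its static mesh component and the ball's mesh.
; The result is only printed to screen as debug text, and the default BeginPlay, overlap and Tick events are disabled stubs.
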(event `DistanceTo GolfBall`
  (params (ActorClass :type "Actor Class Reference"))
  (bind _returnvalue (`GameplayStatics.GetActorOfClass` ActorClass))
  (`KismetSystemLibrary.PrintString` (`KismetStringLibrary.Conv_DoubleToString` (`KismetMathLibrary.Vector_Distance2D` (`SceneComponent.K2_GetComponentLocation` (`self.GetComponentByClass` _returnvalue "/Script/Engine.StaticMeshComponent")) (`SceneComponent.K2_GetComponentLocation` (`self.StaticMesh`)))) true true (struct :`G` 0.66 :`B` 1.0 :`A` 1.0) 30.0))

(fn `UserConstructionScript`
  (`parent.UserConstructionScript`))