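; Player character for a ball-throwing game, with movement, look, jump and an action bar of throwable objects.
; Number keys set the GrabbedBall class and highlight it in WB_UI; right-click spawns it with an impulse scaled by adjustable Speed.
; Left Ctrl places a single stick, and F line-traces to destroy nearby "ball"-tagged actors, clearing the stick flag.
; Spawning and destruction go through OS_ events; E only prints trace hits, and DropBall is unwired.
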(event `InputAxis|Forward/Backward`
  (params (AxisValue :type "Float (single-precision)"))
  ;[0 0 0] Character Movement
  (`self.AddMovementInput` (`KismetMathLibrary.GetForwardVector` (`KismetMathLibrary.MakeRotator` 0.0 0.0 (.yaw (`self.GetControlRotation`)))) AxisValue))

(event `InputAxis|Right/Left`
  (params (AxisValue :type "Float (single-precision)"))
  ;[0 0 0] Character Movement
  (`self.AddMovementInput` (`KismetMathLibrary.GetRightVector` (`KismetMathLibrary.MakeRotator` 0.0 0.0 (.yaw (`self.GetControlRotation`)))) AxisValue))

(event `InputAxis|LookUp/LookDown`
  (params (AxisValue :type "Float (single-precision)"))
  (bind _target (`self.Target`))
  ;[0 0 0] Character Movement
  (`self.AddControllerPitchInput` (`KismetMathLibrary.FClamp` AxisValue -1.0))
  (`PhysicsHandleComponent.SetTargetLocation` (`self.PhysicsHandle`) (+ (`SceneComponent.K2_GetComponentLocation` _target) (`KismetMathLibrary.GetForwardVector` (`SceneComponent.K2_GetComponentRotation` _target)))))

(event `InputAxis|LookRight/LookLeft`
  (params (AxisValue :type "Float (single-precision)"))
  (bind _target (`self.Target`))
  ;[0 0 0] Character Movement
  (`self.AddControllerYawInput` (`KismetMathLibrary.FClamp` AxisValue -1.0))
  (`PhysicsHandleComponent.SetTargetLocation` (`self.PhysicsHandle`) (+ (`SceneComponent.K2_GetComponentLocation` _target) (`KismetMathLibrary.GetForwardVector` (`SceneComponent.K2_GetComponentRotation` _target)))))

(event `OS_DestroyBall`
  (params (Target :type "Actor Object Reference") (GrabbedBall :type "Actor Class Reference"))
  ;[1 1 1] Character Actions
  (`self.K2_DestroyActor` Target))

(event `OS_DropBall`
  ;[1 1 1] Character Actions
  (`|SpawnActorFromClass` (`self.GrabbedBall`) (`KismetMathLibrary.MakeTransform` (`SceneComponent.K2_GetComponentLocation` (`self.Target`))) "Undefined" "MultiplyWithRoot" null null)
  (set `self.GrabbedBall` null))

(event `Key|F`
  (params (Key :type "Key Structure"))
  (bind _camera (`self.Camera`))
  (bind _returnvalue (`SceneComponent.K2_GetComponentLocation` _camera))
  ;[1 1 1] Character Actions
  (:`Pressed`
    (if (not (`self.HoldingBall`))
      (bind (_outhit _returnvalue_2) (`KismetSystemLibrary.LineTraceSingle` :`Start` _returnvalue :`End` (+ _returnvalue (* (`KismetMathLibrary.GetForwardVector` (`SceneComponent.K2_GetComponentRotation` _camera)) 500.0)) :`TraceChannel` "TraceTypeQuery1" :`DrawDebugType` "ForDuration"))
      (if _returnvalue_2
        (bind (_bblockinghit _binitialoverlap _time _distance _location _impactpoint _normal _impactnormal _physmat _hitactor) (`GameplayStatics.BreakHitResult` _outhit))
        (if (`self.ActorHasTag` _hitactor "ball")
          (if (<= (`KismetMathLibrary.Vector_Distance` _location _returnvalue) 175.0)
            (`self.OS_DestroyBall` _hitactor (`GameplayStatics.GetObjectClass` _hitactor))
            (if (`self.StickOnGround`)
              (set `self.StickOnGround` false)
              (bind _foundwidgets (`WidgetBlueprintLibrary.GetAllWidgetsOfClass` "/Game/WB_UI.WB_UI_C"))
              (`Widget.SetVisibility` (`/Game/WB_UI.Stick_On` (`|GetArrayItem` _foundwidgets)) "Hidden"))))))))

(event `OS_ThrowBall`
  (params (`Spawn Transform Location` :type "Vector Structure") (`Spawn Transform Rotation` :type "Rotator Structure") (Impulse :type "Vector Structure"))
  ;[1 1 1] Character Actions
  (bind _returnvalue (`|SpawnActorFromClass` (`self.GrabbedBall`) (`KismetMathLibrary.MakeTransform` `Spawn Transform Location` `Spawn Transform Rotation`) "AlwaysSpawn" "MultiplyWithRoot" null null))
  (`PrimitiveComponent.AddImpulse` (`self.GetComponentByClass` _returnvalue "/Script/Engine.PrimitiveComponent") Impulse "None" false)
  (set `self.GrabbedBall` null))

(event `Key|RightMouseButton`
  (params (Key :type "Key Structure"))
  (bind _target (`self.Target`))
  (bind _returnvalue (`SceneComponent.K2_GetComponentLocation` _target))
  ;[1 1 1] Character Actions
  (:`Pressed`
    (if (`self.HoldingBall`)
      (`KismetSystemLibrary.PrintString` "Hello")
      (if (`KismetSystemLibrary.IsValidClass` (`self.GrabbedBall`))
        (`self.OS_ThrowBall` _returnvalue (`SceneComponent.K2_GetComponentRotation` _target) (* (`KismetMathLibrary.GetDirectionUnitVector` (`self.K2_GetActorLocation`) _returnvalue) (`self.Speed`)))
        (`Widget.SetVisibility` (`self.ActionBarSelection`) "Hidden")
        (set `self.HoldingBall` false)))))

(event `Key|E`
  (params (Key :type "Key Structure"))
  (bind _camera (`self.Camera`))
  (bind _returnvalue (`SceneComponent.K2_GetComponentLocation` _camera))
  ;[1 1 1] Character Actions
  (:`Pressed`
    (bind (_outhit _returnvalue_2) (`KismetSystemLibrary.LineTraceSingle` :`Start` _returnvalue :`End` (+ _returnvalue (* (`KismetMathLibrary.GetForwardVector` (`SceneComponent.K2_GetComponentRotation` _camera)) 500.0)) :`TraceChannel` "TraceTypeQuery1" :`DrawDebugType` "ForDuration"))
    (if _returnvalue_2
      (`KismetSystemLibrary.PrintString` (`KismetSystemLibrary.GetDisplayName` (`self.GetOwner` (`.HitActor` (`GameplayStatics.BreakHitResult` _outhit))))))))

(event `Key|Add`
  (params (Key :type "Key Structure"))
  (bind _returnvalue (+ (`self.Speed`) 150.0))
  ;[1 1 1] Character Actions
  ;;[1 1 1] Change Speed of Throw
  (:`Released`
    (if (< _returnvalue 1501.0)
      (set `self.Speed` _returnvalue)
      (cast `/Game/Blueprints/NewHUD` (`PlayerController.GetHUD` (`GameplayStatics.GetPlayerController` 0)) :!label _label))))

(event `Key|Subtract`
  (params (Key :type "Key Structure"))
  (bind _returnvalue (- (`self.Speed`) 150.0))
  ;[1 1 1] Character Actions
  ;;[1 1 1] Change Speed of Throw
  (:`Released`
    (if (> _returnvalue -1.0)
      (set `self.Speed` _returnvalue)
      (goto _label))))

(event `InputAction|Jump`
  (params (Key :type "Key Structure"))
  ;[1 1 1] Character Actions
  (:`Pressed`
    (`self.Jump`)))

(event `Key|LeftControl`
  (params (Key :type "Key Structure"))
  (bind _target (`self.Target`))
  ;[1 1 1] ActionBar Code
  (:`Pressed`
    (`self.ActionBarUpdate`)
    (if (not (`self.StickOnGround`))
      (set `self.GrabbedBall` "/Game/Sticks/DefaultStick_01/BP_DefaultStick_01.BP_DefaultStick_01_C")
      (`self.OS_ThrowBall` (`SceneComponent.K2_GetComponentLocation` _target) (`SceneComponent.K2_GetComponentRotation` _target))
      (set `self.StickOnGround` true)
      (bind _foundwidgets (`WidgetBlueprintLibrary.GetAllWidgetsOfClass` "/Game/WB_UI.WB_UI_C"))
      (`Widget.SetVisibility` (`/Game/WB_UI.Stick_On` (`|GetArrayItem` _foundwidgets)) "Visible"))))

(event `Key|One`
  (params (Key :type "Key Structure"))
  ;[1 1 1] ActionBar Code
  (:`Pressed`
    (`self.ActionBarUpdate`)
    (set `self.GrabbedBall` "/Game/Balls/GolfBall_01/BP_GolfBall_01.BP_GolfBall_01_C")
    (bind _foundwidgets (`WidgetBlueprintLibrary.GetAllWidgetsOfClass` "/Game/WB_UI.WB_UI_C"))
    (bind _output_get (set `self.ActionBarSelection` (`/Game/WB_UI.GolfBall_On` (`|GetArrayItem` _foundwidgets))))
    (`Widget.SetVisibility` _output_get "Visible")
    (set `self.HoldingBall` true :!label _label_2)))

(event `Key|Two`
  (params (Key :type "Key Structure"))
  ;[1 1 1] ActionBar Code
  (:`Pressed`
    (`self.ActionBarUpdate`)
    (set `self.GrabbedBall` "/Game/Balls/BocceBall_01/BP_BocceBall_01_Blue.BP_BocceBall_01_Blue_C")
    (bind _foundwidgets (`WidgetBlueprintLibrary.GetAllWidgetsOfClass` "/Game/WB_UI.WB_UI_C"))
    (bind _output_get (set `self.ActionBarSelection` (`/Game/WB_UI.BocceBall_On` (`|GetArrayItem` _foundwidgets))))
    (`Widget.SetVisibility` _output_get "Visible")
    (goto _label_2)))

(event `Key|Three`
  (params (Key :type "Key Structure"))
  ;[1 1 1] ActionBar Code
  (:`Pressed`
    (`self.ActionBarUpdate`)
    (set `self.GrabbedBall` "/Game/Balls/BowlingBall_01/BP_BowlingBall_01.BP_BowlingBall_01_C")
    (bind _foundwidgets (`WidgetBlueprintLibrary.GetAllWidgetsOfClass` "/Game/WB_UI.WB_UI_C"))
    (bind _output_get (set `self.ActionBarSelection` (`/Game/WB_UI.BowlingBall_On` (`|GetArrayItem` _foundwidgets))))
    (`Widget.SetVisibility` _output_get "Visible")
    (goto _label_2)))

(event `Key|Four`
  (params (Key :type "Key Structure"))
  ;[1 1 1] ActionBar Code
  (:`Pressed`
    (`self.ActionBarUpdate`)
    (set `self.GrabbedBall` "/Game/Balls/DrunkenPineapple_01/BP_DrunkenPineapple_01.BP_DrunkenPineapple_01_C")
    (bind _foundwidgets (`WidgetBlueprintLibrary.GetAllWidgetsOfClass` "/Game/WB_UI.WB_UI_C"))
    (bind _output_get (set `self.ActionBarSelection` (`/Game/WB_UI.DrunkenPineapple_On` (`|GetArrayItem` _foundwidgets))))
    (`Widget.SetVisibility` _output_get "Visible")
    (goto _label_2)))

(event `Key|Five`
  (params (Key :type "Key Structure"))
  ;[1 1 1] ActionBar Code
  (:`Pressed`
    (`self.ActionBarUpdate`)
    (set `self.GrabbedBall` "/Game/Balls/Frisbee_01/BP_Frisbee_01.BP_Frisbee_01_C")
    (bind _foundwidgets (`WidgetBlueprintLibrary.GetAllWidgetsOfClass` "/Game/WB_UI.WB_UI_C"))
    (bind _output_get (set `self.ActionBarSelection` (`/Game/WB_UI.Frisbee_On` (`|GetArrayItem` _foundwidgets))))
    (`Widget.SetVisibility` _output_get "Visible")
    (goto _label_2)))

(event `Key|Six`
  (params (Key :type "Key Structure"))
  ;[1 1 1] ActionBar Code
  (:`Pressed`
    (`self.ActionBarUpdate`)
    (set `self.GrabbedBall` "/Game/Balls/Shuttlecock_01/BP_Shuttlecock_01.BP_Shuttlecock_01_C")
    (bind _foundwidgets (`WidgetBlueprintLibrary.GetAllWidgetsOfClass` "/Game/WB_UI.WB_UI_C"))
    (bind _output_get (set `self.ActionBarSelection` (`/Game/WB_UI.Shuttlecock_On` (`|GetArrayItem` _foundwidgets))))
    (`Widget.SetVisibility` _output_get "Visible")
    (goto _label_2)))

(event `Key|Seven`
  (params (Key :type "Key Structure"))
  ;[1 1 1] ActionBar Code
  (:`Pressed`
    (`self.ActionBarUpdate`)
    (set `self.GrabbedBall` "/Game/Balls/StevenSeagull_01/BP_StevenSeagull_01.BP_StevenSeagull_01_C")
    (bind _foundwidgets (`WidgetBlueprintLibrary.GetAllWidgetsOfClass` "/Game/WB_UI.WB_UI_C"))
    (bind _output_get (set `self.ActionBarSelection` (`/Game/WB_UI.StevenSeagull_On` (`|GetArrayItem` _foundwidgets))))
    (`Widget.SetVisibility` _output_get "Visible")
    (goto _label_2)))

(event `Key|Eight`
  (params (Key :type "Key Structure"))
  ;[1 1 1] ActionBar Code
  (:`Pressed`
    (`self.ActionBarUpdate`)
    (set `self.GrabbedBall` "/Game/Balls/GolfBall_01/BP_GolfBall_01_Pink.BP_GolfBall_01_Pink_C")
    (bind _foundwidgets (`WidgetBlueprintLibrary.GetAllWidgetsOfClass` "/Game/WB_UI.WB_UI_C"))
    (bind _output_get (set `self.ActionBarSelection` (`/Game/WB_UI.PinkBall_On` (`|GetArrayItem` _foundwidgets))))
    (`Widget.SetVisibility` _output_get "Visible")
    (goto _label_2)))

(fn `ActionBarUpdate`
  (bind _actionbarselection (`self.ActionBarSelection`) ; Check if something is selected
    (:`then`
      (`Widget.SetVisibility` _actionbarselection "Hidden"))
    (:`else`)))

(fn `UserConstructionScript`)