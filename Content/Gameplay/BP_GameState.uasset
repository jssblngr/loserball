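; Game state Blueprint that keeps the ball selection UI in sync with the balls currently held.
; Every Tick it looks up the BallSelection_01 widget and walks the children of its BallListGrid.
; Children whose display name matches a held ball's class name are disabled.
; Children are re-enabled only once HeldBalls is completely empty, so releasing one of several balls leaves its button disabled.
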(event `self.ReceiveTick`
  (params (DeltaSeconds :type "Float (single-precision)"))
  (bind _heldballs (`self.HeldBalls`))
  (if (`KismetArrayLibrary.Array_IsNotEmpty` _heldballs)
    (for _array_element _heldballs
      (bind _foundwidgets (`WidgetBlueprintLibrary.GetAllWidgetsOfClass` "/Game/Menus/BallSelection_01.BallSelection_01_C" false))
      (if (`KismetArrayLibrary.Array_IsValidIndex` _foundwidgets)
        (bind _returnvalue (`PanelWidget.GetAllChildren` (`/Game/Menus/BallSelection_01.BallListGrid` (`|GetArrayItem` _foundwidgets))))
        (if (`KismetArrayLibrary.Array_IsValidIndex` _returnvalue)
          (for _array_element_2 _returnvalue
            (if (`KismetStringLibrary.EqualEqual_StrStr` (`KismetSystemLibrary.GetClassDisplayName` _array_element) (`KismetSystemLibrary.GetDisplayName` _array_element_2))
              (`Widget.SetIsEnabled` _array_element_2 false))))))
    (else
      (bind _foundwidgets_2 (`WidgetBlueprintLibrary.GetAllWidgetsOfClass` "/Game/Menus/BallSelection_01.BallSelection_01_C"))
      (if (`KismetArrayLibrary.Array_IsValidIndex` _foundwidgets_2)
        (for _array_element_3 (`PanelWidget.GetAllChildren` (`/Game/Menus/BallSelection_01.BallListGrid` (`|GetArrayItem` _foundwidgets_2)))
          (switch `string` (`KismetSystemLibrary.GetDisplayName` _array_element_3)
            (:`Default`
              (`Widget.SetIsEnabled` _array_element_3 true))))))))

(fn `UserConstructionScript`)