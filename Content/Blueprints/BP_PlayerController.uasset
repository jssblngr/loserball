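; Player controller that creates a session lobby through BP_GameInstance on BeginPlay, then switches to game-only input with a hidden cursor.
; Escape opens the PauseMenu widget with UI-only input and a visible cursor.
; Holding L reveals ball locations by calling ShowLocation on every PhysicsAsset and BP_StevenSeagull_01 actor, and releasing it calls HideLocation on them.
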(event `self.ReceiveBeginPlay`
  (bind _asbp_game_instance (cast `/Game/Blueprints/BP_GameInstance` (`GameplayStatics.GetGameInstance`)))
  (`/Game/Blueprints/BP_GameInstance.CreateSessionLobby` _asbp_game_instance)
  (set `self.bShowMouseCursor` false)
  (`WidgetBlueprintLibrary.SetInputMode_GameOnly` self)
  (set `self.Lobby?` false))

(event `Key|Escape`
  (params (Key :type "Key Structure"))
  (bind _returnvalue (`GameplayStatics.GetPlayerController` 0))
  ;[1 1 1] Pause Game
  (:`Pressed`
    (bind _returnvalue_2 (`|CreateWidget` "/Game/Blueprints/UI/PauseMenu.PauseMenu_C"))
    (`UserWidget.AddToViewport` _returnvalue_2 0)
    (`WidgetBlueprintLibrary.SetInputMode_UIOnlyEx` _returnvalue _returnvalue_2 "DoNotLock" true)
    (set `PlayerController.bShowMouseCursor` true _returnvalue)))

(event `Key|L`
  (params (Key :type "Key Structure"))
  ;[1 1 1] Show Ball Location
  (:`Pressed`
    (bind _outactors (`GameplayStatics.GetAllActorsOfClass` "/Game/Blueprints/PhysicsAsset.PhysicsAsset_C"))
    (for _array_element _outactors
      (`/Game/Blueprints/PhysicsAsset.ShowLocation` _array_element))
    (bind _outactors_2 (`GameplayStatics.GetAllActorsOfClass` "/Game/Balls/StevenSeagull_01/BP_StevenSeagull_01.BP_StevenSeagull_01_C"))
    (for _array_element_2 _outactors_2
      (`/Game/Balls/StevenSeagull_01/BP_StevenSeagull_01.ShowLocation` _array_element_2)))
  (:`Released`
    (bind _outactors_3 (`GameplayStatics.GetAllActorsOfClass` "/Game/Blueprints/PhysicsAsset.PhysicsAsset_C"))
    (for _array_element_3 _outactors_3
      (`/Game/Blueprints/PhysicsAsset.HideLocation` _array_element_3))
    (bind _outactors_4 (`GameplayStatics.GetAllActorsOfClass` "/Game/Balls/StevenSeagull_01/BP_StevenSeagull_01.BP_StevenSeagull_01_C"))
    (for _array_element_4 _outactors_4
      (`/Game/Balls/StevenSeagull_01/BP_StevenSeagull_01.HideLocation` _array_element_4))))

(fn `UserConstructionScript`)