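; Blueprint function library that changes a ball's physics damping based on the surface material it hits.
; Each function compares the hit's physical material against sand, grass and dirt, then sets linear and angular damping, with sand damping hardest.
; Separate versions handle static and skeletal meshes.
; Other surfaces leave the current damping unchanged, as neither function resets it.
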(fn `FN_PhysicalMaterialCheck`
  (params (Hit :type "HitResult Structure") (StaticMesh :type "StaticMeshComponent Object Reference"))
  (bind (_bblockinghit _binitialoverlap _time _distance _location _impactpoint _normal _impactnormal _physmat) (`GameplayStatics.BreakHitResult` Hit))
  (if (== _physmat "/Game/Materials/0_Physical_Materials/PM_Sand_01.PM_Sand_01")
    (`PrimitiveComponent.SetLinearDamping` StaticMesh 3.0)
    (`PrimitiveComponent.SetAngularDamping` StaticMesh 3.0)
    (elif (== _physmat "/Game/Materials/0_Physical_Materials/PM_Grass_01.PM_Grass_01")
      (`PrimitiveComponent.SetLinearDamping` StaticMesh 2.0)
      (`PrimitiveComponent.SetAngularDamping` StaticMesh 2.0)
      (elif (== _physmat "/Game/Materials/0_Physical_Materials/PM_Dirt_01.PM_Dirt_01")
        (`PrimitiveComponent.SetLinearDamping` StaticMesh 2.0)
        (`PrimitiveComponent.SetAngularDamping` StaticMesh 2.0)))))

(fn `FN_PhysicalMaterialCheck_SkeletalMesh`
  (params (Hit :type "HitResult Structure") (SkeletalMesh :type "SkeletalMeshComponent Object Reference"))
  (bind (_bblockinghit _binitialoverlap _time _distance _location _impactpoint _normal _impactnormal _physmat) (`GameplayStatics.BreakHitResult` Hit))
  (if (== _physmat "/Game/Materials/0_Physical_Materials/PM_Sand_01.PM_Sand_01")
    (`PrimitiveComponent.SetLinearDamping` SkeletalMesh 3.0)
    (`PrimitiveComponent.SetAngularDamping` SkeletalMesh 3.0)
    (elif (== _physmat "/Game/Materials/0_Physical_Materials/PM_Grass_01.PM_Grass_01")
      (`PrimitiveComponent.SetLinearDamping` SkeletalMesh 2.0)
      (`PrimitiveComponent.SetAngularDamping` SkeletalMesh 2.0)
      (elif (== _physmat "/Game/Materials/0_Physical_Materials/PM_Dirt_01.PM_Dirt_01")
        (`PrimitiveComponent.SetLinearDamping` SkeletalMesh 2.0)
        (`PrimitiveComponent.SetAngularDamping` SkeletalMesh 2.0)))))