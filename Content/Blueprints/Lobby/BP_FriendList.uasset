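; BP_FriendList is a lobby actor for the friend list, shown for one player platform at a time and hidden when the mouse strays.
; Show toggles visibility, tells the previous platform to turn off its friend list, and tracks the requesting one.
; Each tick while visible, it projects the mouse ray to the actor's distance and hides if that point falls outside FalloffRadius of the actor.
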(event `self.ReceiveTick`
  (params (DeltaSeconds :type "Float (single-precision)"))
  (`self.CheckToHideFriendList`))

(fn `CheckToHideFriendList`
  (bind _returnvalue (`self.K2_GetActorLocation`))
  (bind (_worldlocation _worlddirection) (`PlayerController.DeprojectMousePositionToWorld` (`GameplayStatics.GetPlayerController` 0)))
  (if (`self.bHidden`)
    _
    (elif (not (== (+ _worldlocation (* _worlddirection (`KismetMathLibrary.Vector_Distance` _returnvalue _worldlocation))) _returnvalue :`ErrorTolerance` (`self.FalloffRadius`)))
      (`self.Show` false))))

(fn `Show`
  (params (Show :type Boolean) (FromLobbyPlayerPlatform :type "/Game/Blueprints/Lobby/BP_LobbyPlayerPlatform Object Reference"))
  (bind _lastlobbyplayerplatform (`self.LastLobbyPlayerPlatform`))
  (bind _lastlobbyplayerplatform_2 (`self.LastLobbyPlayerPlatform`))
  (if Show
    (`self.SetActorHiddenInGame` false)
    (`/Engine/EditorBlueprintResources/StandardMacros.IsValid` _lastlobbyplayerplatform_2
      (:`Is Valid`
        (`/Game/Blueprints/Lobby/BP_LobbyPlayerPlatform.ShowFriendList` _lastlobbyplayerplatform_2 false))
      (:`Is Not Valid`
        _))
    (set `self.LastLobbyPlayerPlatform` FromLobbyPlayerPlatform)
    (else
      (`self.SetActorHiddenInGame` true)
      (`/Engine/EditorBlueprintResources/StandardMacros.IsValid` _lastlobbyplayerplatform
        (:`Is Valid`
          (`/Game/Blueprints/Lobby/BP_LobbyPlayerPlatform.ShowFriendList` _lastlobbyplayerplatform false))
        (:`Is Not Valid`
          _))
      (set `self.LastLobbyPlayerPlatform` null))))

(fn `UserConstructionScript`)