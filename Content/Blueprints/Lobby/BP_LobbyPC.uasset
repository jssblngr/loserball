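; Lobby player controller that creates the lobby UI for the local player and reports that player's lobby info to BP_LobbyGM.
; BeginPlay runs that setup, pushes the info to the game mode and asks BP_GameInstance to create a session.
; Server-named events toggle ready status or resend info, with a short-delay retry event.
; Match start shows the loading screen and disables input; T and R keys print debug strings.
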(event `ToggleReadyStatusOnServer`
  (bind _playerlobbyinfopc (`self.PlayerLobbyInfoPC`))
  (setmembers `/Game/Blueprints/Lobby/S_PlayerLobbyInfo` :`StructRef` _playerlobbyinfopc :`bReady` (not (`.bReady_10_FE2C43E146D8B9F91EF667B0D9393627` (break `/Game/Blueprints/Lobby/S_PlayerLobbyInfo` _playerlobbyinfopc))))
  (bind _asbp_lobby_gm (cast `/Game/Blueprints/Lobby/BP_LobbyGM` (`GameplayStatics.GetGameMode`))
    (:`then`
      (`/Game/Blueprints/Lobby/BP_LobbyGM.UpdatePlayerLobbyInfo` _asbp_lobby_gm self))
    (:`CastFailed`
      (`KismetSystemLibrary.PrintString` "CAST FAILED"))))

(event `SetPlayerNameOnServer`
  (bind _asbp_lobby_gm (cast `/Game/Blueprints/Lobby/BP_LobbyGM` (`GameplayStatics.GetGameMode`)))
  (`/Game/Blueprints/Lobby/BP_LobbyGM.UpdatePlayerLobbyInfo` _asbp_lobby_gm self))

(event `TryAgainUpdatingLobbyInfo`
  (`KismetSystemLibrary.Delay` 0.1)
  (bind _asbp_lobby_gm (cast `/Game/Blueprints/Lobby/BP_LobbyGM` (`GameplayStatics.GetGameMode`)))
  (`/Game/Blueprints/Lobby/BP_LobbyGM.UpdatePlayerLobbyInfo` _asbp_lobby_gm self))

(event `self.ReceiveBeginPlay`
  (`self.Setup`)
  (bind _asbp_lobby_gm (cast `/Game/Blueprints/Lobby/BP_LobbyGM` (`GameplayStatics.GetGameMode`)))
  (`/Game/Blueprints/Lobby/BP_LobbyGM.UpdatePlayerLobbyInfo` _asbp_lobby_gm self)
  (bind _asbp_game_instance (cast `/Game/Blueprints/BP_GameInstance` (`GameplayStatics.GetGameInstance`)))
  (`/Game/Blueprints/BP_GameInstance.CreateSession` _asbp_game_instance))

(event `OnStartMatch`
  (`/Game/Blueprints/Lobby/WB_LobbyUI.ShowLoadingScreen` (`self.LobbyUIRef`))
  (`self.DisableInput` self))

(event `Key|T`
  (params (Key :type "Key Structure"))
  (:`Pressed`
    (`KismetSystemLibrary.PrintString` (`AdvancedSessionsLibrary.GetCurrentSessionID_AsString`))))

(event `Key|R`
  (params (Key :type "Key Structure"))
  (:`Pressed`
    (`KismetSystemLibrary.PrintString` "Hello")))

(fn `Setup`
  (if (`self.IsLocalPlayerController`)
    (set `self.bShowMouseCursor` true)
    (`WidgetBlueprintLibrary.SetInputMode_GameAndUIEx` self null "DoNotLock" false)
    (bind _returnvalue (`|CreateWidget` "/Game/Blueprints/Lobby/WB_LobbyUI.WB_LobbyUI_C"))
    (bind _output_get (set `self.LobbyUIRef` _returnvalue))
    (`UserWidget.AddToViewport` _output_get 0)
    (`self.SetPlayerNameOnServer`)))

(fn `UserConstructionScript`)