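; Physics-driven static mesh actor in a golf game that reports its movement state and distance to the golf ball through debug prints.
; Outside the lobby, a looping timer polls rigid body sleep state, printing a missing-ball message once when awake and the distance to the first BP_GolfBall_01 once when asleep.
; Mesh hits feed a physical material check.
; ShowLocation and HideLocation spawn and destroy a location marker actor at the mesh.
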(event `self.ReceiveBeginPlay`
  (bind _asbp_player_controller (cast `/Game/Blueprints/BP_PlayerController` (`GameplayStatics.GetPlayerController` 0)))
  (if (not (`/Game/Blueprints/BP_PlayerController.Lobby?` _asbp_player_controller))
    (`KismetSystemLibrary.K2_SetTimerDelegate` (delegate `Testting`) 0.5 true)))

(event `Testting`
  (if (`PrimitiveComponent.IsAnyRigidBodyAwake` (`self.StaticMesh`))
    (`/Engine/EditorBlueprintResources/StandardMacros.DoOnce` false
      (:`Completed`
        (`KismetSystemLibrary.PrintString` "Golf Ball is Missing!" true true (struct :`R` 1.0 :`A` 1.0) 30.0)))
    (else
      (`/Engine/EditorBlueprintResources/StandardMacros.DoOnce` false
        (:`Completed`
          (bind _outactors (`GameplayStatics.GetAllActorsOfClass` "/Game/Balls/GolfBall_01/BP_GolfBall_01.BP_GolfBall_01_C"))
          (bind _output (`|GetArrayItem` _outactors))
          (`/Engine/EditorBlueprintResources/StandardMacros.IsValid` _output
            (:`Is Valid`
              (`KismetSystemLibrary.PrintString` (`KismetStringLibrary.Conv_DoubleToString` (`KismetMathLibrary.Vector_Distance` (`SceneComponent.K2_GetComponentLocation` (`/Game/Blueprints/PhysicsAsset.StaticMesh` _output)) (`SceneComponent.K2_GetComponentLocation` (`self.StaticMesh`)))) true true (struct :`G` 0.66 :`B` 1.0 :`A` 1.0) 32.0))))))))

(event `self.StaticMesh.OnComponentHit`
  (params (HitComponent :type "PrimitiveComponent Object Reference") (OtherActor :type "Actor Object Reference") (OtherComp :type "PrimitiveComponent Object Reference") (NormalImpulse :type "Vector Structure") (Hit :type "HitResult Structure (by ref)"))
  (`/Game/Blueprints/Functions/BallFunctionLibrary.FN_PhysicalMaterialCheck` Hit (`self.StaticMesh`)))

(event `ShowLocation`
  (bind _returnvalue (`|SpawnActorFromClass` "/Game/VFX/BallLocation_01/BP_BallLocation_01_A.BP_BallLocation_01_A_C" (`KismetMathLibrary.MakeTransform` (`SceneComponent.K2_GetComponentLocation` (`self.StaticMesh`))) "Undefined" "MultiplyWithRoot" null null)))

(event `HideLocation`
  (`/Engine/EditorBlueprintResources/StandardMacros.IsValid` (stale `ShowLocation` _returnvalue)
    (:`Is Valid`
      (`self.K2_DestroyActor` (stale `ShowLocation` _returnvalue)))))

(fn `NewFunction`
  (`KismetSystemLibrary.PrintString` "Hello"))

(fn `UserConstructionScript`)