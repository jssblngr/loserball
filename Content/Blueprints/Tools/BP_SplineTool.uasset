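; Spline tool actor that builds a chain of deformed static meshes along an editable spline.
; The construction script adds a spline mesh component per SectionLength interval, taking positions and tangents by distance and clamping tangent size to the section length.
; A SnapToGround event line-traces straight down from each spline point on the Visibility channel and moves the point to the impact location.
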(event `SnapToGround`
  (bind _spline (`self.Spline`))
  (for _index (range (+ (`SplineComponent.GetNumberOfSplinePoints` _spline) 1))
    (bind (_returnvalue_x _returnvalue_y _returnvalue_z) (`KismetMathLibrary.BreakVector` (`SplineComponent.GetLocationAtSplinePoint` _spline _index "World")))
    (bind _outhit (`KismetSystemLibrary.LineTraceSingle` :`Start` (`KismetMathLibrary.MakeVector` _returnvalue_x _returnvalue_y _returnvalue_z) :`End` (`KismetMathLibrary.MakeVector` _returnvalue_x _returnvalue_y (- _returnvalue_z 1000000.0)) :`TraceChannel` "TraceTypeQuery1" :`DrawDebugType` "ForOneFrame"))
    (`SplineComponent.SetLocationAtSplinePoint` _spline _index (`.ImpactPoint` (`GameplayStatics.BreakHitResult` _outhit)) "World" true)))

(fn `UserConstructionScript`
  (bind _sectionlength (`self.SectionLength`))
  (bind _spline (`self.Spline`))
  (for _index (range (+ (`KismetMathLibrary.FTrunc` (/ (`SplineComponent.GetSplineLength` (`self.Spline`)) (`self.SectionLength`))) 1))
    (bind _returnvalue (`AddComponent|NODE_AddSplineMeshComponent-0`))
    (`StaticMeshComponent.SetStaticMesh` _returnvalue (`self.Spline Mesh`))
    (`SplineMeshComponent.SetForwardAxis` _returnvalue "X" true)
    (bind _returnvalue_2 (* _index _sectionlength))
    (bind _returnvalue_3 (* (+ _index 1) _sectionlength))
    (`SplineMeshComponent.SetStartAndEnd` _returnvalue (`SplineComponent.GetLocationAtDistanceAlongSpline` _spline _returnvalue_2 "Local") (`KismetMathLibrary.ClampVectorSize` (`SplineComponent.GetTangentAtDistanceAlongSpline` _spline _returnvalue_2 "Local") 0.0 _sectionlength) (`SplineComponent.GetLocationAtDistanceAlongSpline` _spline _returnvalue_3 "Local") (`KismetMathLibrary.ClampVectorSize` (`SplineComponent.GetTangentAtDistanceAlongSpline` _spline _returnvalue_3 "Local") 0.0 _sectionlength) true)))